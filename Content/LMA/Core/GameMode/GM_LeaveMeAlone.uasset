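; GM_LeaveMeAlone is a game mode that runs the match countdown and ends play when time runs out.
; BeginPlay starts a looping one-second timer that decrements GameTime.
; At zero it clears the timer, pauses the game, shows the WBP_TimeOver widget and switches PC_LeaveMeAlone to UI-only input with a visible cursor.
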(event `self.ReceiveBeginPlay`
  (bind _returnvalue (`KismetSystemLibrary.K2_SetTimerDelegate` (delegate `CustomEvent`) 1.0 true))
  (set `self.Game Timer Handle` _returnvalue))

(event `CustomEvent`
  (bind _output_get (set `self.Game Time` (- (`self.Game Time`) 1)))
  (if (== _output_get 0)
    (`KismetSystemLibrary.K2_ClearAndInvalidateTimerHandle` (`self.Game Timer Handle`))
    (`GameplayStatics.SetGamePaused` true)
    (bind _returnvalue (`|CreateWidget` "/Game/LMA/Widgets/UI/WBP_TimeOver.WBP_TimeOver_C"))
    (`UserWidget.AddToViewport` _returnvalue 0)
    (bind _aspc_leave_me_alone (cast `/Game/LMA/Core/Controller/PC_LeaveMeAlone` (`GameplayStatics.GetPlayerController` 0)))
    (`WidgetBlueprintLibrary.SetInputMode_UIOnlyEx` _aspc_leave_me_alone _returnvalue)
    (set `PlayerController.bShowMouseCursor` true _aspc_leave_me_alone)))

(fn `UserConstructionScript`)