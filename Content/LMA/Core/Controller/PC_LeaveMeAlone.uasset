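; Player controller for LeaveMeAlone that opens the pause and game-over screens.
; From BeginPlay it listens for possessed pawn changes, treating any change as game over after a short delay.
; The Pause input is guarded by a Paused flag, which this graph never clears.
; Both paths pause the game, show their widget, switch to UI-only input and reveal the cursor.
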(event `self.ReceiveBeginPlay`
  (add `self.OnPossessedPawnChanged` (delegate `OnPossessedPawnChanged_Event`)))

(event `OnPossessedPawnChanged_Event` :!signature `self.OnPossessedPawnChanged`
  (params (OldPawn :type "Pawn Object Reference") (NewPawn :type "Pawn Object Reference"))
  (bind _returnvalue (`GameplayStatics.GetPlayerController` 0))
  (`KismetSystemLibrary.Delay` 1.25)
  (`GameplayStatics.SetGamePaused` true)
  (bind _returnvalue_2 (`|CreateWidget` "/Game/LMA/Widgets/UI/WBP_GameOver.WBP_GameOver_C"))
  (bind _output_get (set `self.Death Widget` _returnvalue_2))
  (`UserWidget.AddToViewport` _output_get 0)
  (`WidgetBlueprintLibrary.SetInputMode_UIOnlyEx` _returnvalue _output_get)
  (set `PlayerController.bShowMouseCursor` true _returnvalue))

(event `InputAction|Pause`
  (params (Key :type "Key Structure"))
  (:`Pressed`
    (if (not (`self.Paused`))
      (set `self.Paused` true)
      (`GameplayStatics.SetGamePaused` true)
      (bind _returnvalue (`|CreateWidget` "/Game/LMA/Widgets/UI/WBP_Pause.WBP_Pause_C"))
      (bind _output_get (set `self.Pause Widget` _returnvalue))
      (`UserWidget.AddToViewport` _output_get 0)
      (`WidgetBlueprintLibrary.SetInputMode_UIOnlyEx` self _output_get)
      (set `self.bShowMouseCursor` true))))

(fn `UserConstructionScript`)